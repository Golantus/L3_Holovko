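; A push-button actor that spawns a straight-movement product through its creator when the player presses it.
; Overlapping its box as the third-person character enables input and opens a gate for the PushButton action; leaving closes the gate.
; A press plays timelines that lerp the button in and back out, then asks MyCreator to spawn a BP_StraightMovementProduct with fixed start and end points, only if none currently exists.
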(event `self.ReceiveBeginPlay`
  (`parent.ReceiveBeginPlay`))

(event `InputAction|PushButton`
  (params (Key :type "Key Structure"))
  ;[1 1 1] Push Button
  (:`Pressed`
    (`/Engine/EditorBlueprintResources/StandardMacros.Gate` true :!label _label
      (:`Exit`
        (bind (_direction _buttonin) (`Timeline|Timeline` :!via `PlayFromStart`)
          (:`Update`
            (`SceneComponent.K2_SetRelativeTransform` (`self.Button`) (`KismetMathLibrary.TLerp` (`self.OutPosition`) (`self.InPosition`) _buttonin) false false))
          (:`Finished`
            (bind (_direction_2 _buttonin_2) (`Timeline|Timeline_0` :!via `ReverseFromEnd`)
              (:`Update`
                (`SceneComponent.K2_SetRelativeTransform` (`self.Button`) (`KismetMathLibrary.TLerp` (`self.OutPosition`) (`self.InPosition`) _buttonin_2) false false))
              (:`Finished`
                ;[1 1 1] SpawnActorFromCreator
                (`/Engine/EditorBlueprintResources/StandardMacros.IsValid` (`self.SpawnedActor`)
                  (:`Is Not Valid`
                    (bind _returnvalue (`Creator.SpawnActor` (`self.MyCreator`)))
                    (bind _asbp_straight_movement_product (cast `/Game/BP_StraightMovementProduct` _returnvalue))
                    (bind _output_get (set `self.SpawnedActor` _asbp_straight_movement_product))
                    (`ConcreteProductStraightMovement.SetStartSettings` _output_get (1000.0 0.0 0.0) (1000.0 0.0 1000.0) 100.0 true)))))))))))

(event `self.Box.OnComponentBeginOverlap`
  (params (OverlappedComponent :type "PrimitiveComponent Object Reference") (OtherActor :type "Actor Object Reference") (OtherComp :type "PrimitiveComponent Object Reference") (OtherBodyIndex :type Integer) (bFromSweep :type Boolean) (SweepResult :type "HitResult Structure (by ref)"))
  ;[1 1 1] Push Button
  (cast `/Game/ThirdPerson/Blueprints/BP_ThirdPersonCharacter` OtherActor)
  (`self.EnableInput` (`GameplayStatics.GetPlayerController` 0))
  (goto _label :!via `Open`))

(event `self.Box.OnComponentEndOverlap`
  (params (OverlappedComponent :type "PrimitiveComponent Object Reference") (OtherActor :type "Actor Object Reference") (OtherComp :type "PrimitiveComponent Object Reference") (OtherBodyIndex :type Integer))
  ;[1 1 1] Push Button
  (cast `/Game/ThirdPerson/Blueprints/BP_ThirdPersonCharacter` OtherActor)
  (goto _label :!via `Close`))

(fn `UserConstructionScript`
  (`parent.UserConstructionScript`))